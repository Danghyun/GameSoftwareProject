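; BP_CheckPoint is a one-time checkpoint that records its location on the player.
; The first BoxCollision overlap, with no check on the overlapping actor, stores the actor location in BP_Player's CheckPoint variable and sets IsActivated to block retriggering.
; It then lights the PointLight, shows and plays a BP_Notification widget, and switches the light off after a short delay.
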(event `self.Box Collision.OnComponentBeginOverlap`
  (params (OverlappedComponent :type "PrimitiveComponent Object Reference") (OtherActor :type "Actor Object Reference") (OtherComp :type "PrimitiveComponent Object Reference") (OtherBodyIndex :type Integer) (bFromSweep :type Boolean) (SweepResult :type "HitResult Structure (by ref)"))
  (if (not (`self.isActivated`))
    (bind _asbp_player (cast `/Game/Blueprints/BP_Player` (`GameplayStatics.GetPlayerCharacter` 0)))
    (set `/Game/Blueprints/BP_Player.CheckPoint` (`self.K2_GetActorLocation`) _asbp_player)
    (set `self.isActivated` true)
    (`LightComponent.SetIntensity` (`self.PointLight`) 500.0)
    (bind _returnvalue (`|CreateWidget` "/Game/Blueprints/Widget/BP_Notification.BP_Notification_C"))
    (`UserWidget.AddToViewport` _returnvalue 0)
    (`/Game/Blueprints/Widget/BP_Notification.Play Notification` _returnvalue)
    (`KismetSystemLibrary.Delay` 5.0)
    (`LightComponent.SetIntensity` (`self.PointLight`) 0.0)))

(fn `UserConstructionScript`)
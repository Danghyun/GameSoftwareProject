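; Elevator actor that moves its EV component vertically when a player inside a trigger box calls for up or down travel.
; DownBox and UpBox show prompt widgets on player overlap and open gates that let GoDown and GoUp through.
; MoveDown lerps EV between hard-coded world positions on the Alpha timeline.
; MoveUp instead reverses a separate Movement timeline, which lerps between the Down and Up component locations.
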(event `Go Down`
  (`/Engine/EditorBlueprintResources/StandardMacros.Gate` true :!label _label
    (:`Exit`
      (`self.Move down`))))

(event `self.Down Box.OnComponentBeginOverlap`
  (params (OverlappedComponent :type "PrimitiveComponent Object Reference") (OtherActor :type "Actor Object Reference") (OtherComp :type "PrimitiveComponent Object Reference") (OtherBodyIndex :type Integer) (bFromSweep :type Boolean) (SweepResult :type "HitResult Structure (by ref)"))
  (cast `/Game/Blueprints/BP_Player` OtherActor)
  (bind _returnvalue (`|CreateWidget` "/Game/Blueprints/Elevator/DownMassage.DownMassage_C"))
  (`UserWidget.AddToViewport` _returnvalue 0)
  (goto _label :!via `Open`))

(event `self.Down Box.OnComponentEndOverlap`
  (params (OverlappedComponent :type "PrimitiveComponent Object Reference") (OtherActor :type "Actor Object Reference") (OtherComp :type "PrimitiveComponent Object Reference") (OtherBodyIndex :type Integer))
  (cast `/Game/Blueprints/BP_Player` OtherActor)
  (`Widget.RemoveFromParent` (stale `self.Down Box.OnComponentBeginOverlap` _returnvalue))
  (goto _label :!via `Close`))

(event `Go Up`
  (`/Engine/EditorBlueprintResources/StandardMacros.Gate` true :!label _label_2
    (:`Exit`
      (`self.Move Up`))))

(event `self.Up Box.OnComponentBeginOverlap`
  (params (OverlappedComponent :type "PrimitiveComponent Object Reference") (OtherActor :type "Actor Object Reference") (OtherComp :type "PrimitiveComponent Object Reference") (OtherBodyIndex :type Integer) (bFromSweep :type Boolean) (SweepResult :type "HitResult Structure (by ref)"))
  (cast `/Game/Blueprints/BP_Player` OtherActor)
  (bind _returnvalue (`|CreateWidget` "/Game/Blueprints/Elevator/UpMassage.UpMassage_C"))
  (`UserWidget.AddToViewport` _returnvalue 0)
  (goto _label_2 :!via `Open`))

(event `self.Up Box.OnComponentEndOverlap`
  (params (OverlappedComponent :type "PrimitiveComponent Object Reference") (OtherActor :type "Actor Object Reference") (OtherComp :type "PrimitiveComponent Object Reference") (OtherBodyIndex :type Integer))
  (cast `/Game/Blueprints/BP_Player` OtherActor)
  (`Widget.RemoveFromParent` (stale `self.Up Box.OnComponentBeginOverlap` _returnvalue))
  (goto _label_2 :!via `Close`))

(event `Move down`
  (bind (_direction _0_to_1) (`Timeline|Movement` :!label _label_3)
    (:`Update`
      (`SceneComponent.K2_SetWorldLocation` (`self.EV`) (`KismetMathLibrary.VLerp` (`SceneComponent.K2_GetComponentLocation` (`self.Down`)) (`SceneComponent.K2_GetComponentLocation` (`self.Up`)) _0_to_1) false false))))

(event `Move Up`
  (goto _label_3 :!via `Reverse`))

(event `Event Move Down`
  (bind (_direction _0_to_1) (`Timeline|Alpha`)
    (:`Update`
      (`SceneComponent.K2_SetWorldLocation` (`self.EV`) (`KismetMathLibrary.VLerp` (7597.999997 -5.000007 99.66421) (7597.999997 5.000011 -197.651761) _0_to_1) false false))))

(fn `UserConstructionScript`)
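; BoxTrigger is a goal trigger volume that stages the game-clear celebration and ending screen.
; Until completed, entering the box shows the Clearmessage widget and calls Firecracker on every FireStarter actor, without filtering what overlapped.
; The first exit sets Complete, then after delays swaps the message for the BP_GameComplete widget, pauses the game and switches to UI-only input with a visible cursor.
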(event `self.Box.OnComponentBeginOverlap`
  (params (OverlappedComponent :type "PrimitiveComponent Object Reference") (OtherActor :type "Actor Object Reference") (OtherComp :type "PrimitiveComponent Object Reference") (OtherBodyIndex :type Integer) (bFromSweep :type Boolean) (SweepResult :type "HitResult Structure (by ref)"))
  (if (not (`self.Complete`))
    (bind _returnvalue (`|CreateWidget` "/Game/Blueprints/Firecracker/Clearmessage.Clearmessage_C"))
    (`UserWidget.AddToViewport` _returnvalue 0)
    (bind _outactors (`GameplayStatics.GetAllActorsOfClass` "/Game/Blueprints/Firecracker/FireStarter.FireStarter_C"))
    (for _array_element _outactors
      (bind _asfire_starter (cast `/Game/Blueprints/Firecracker/FireStarter` _array_element))
      (`/Game/Blueprints/Firecracker/FireStarter.Firecracker` _asfire_starter)
      (`KismetSystemLibrary.PrintString` (`KismetStringLibrary.Conv_BoolToString` (`self.Complete`))))))

(event `self.Box.OnComponentEndOverlap`
  (params (OverlappedComponent :type "PrimitiveComponent Object Reference") (OtherActor :type "Actor Object Reference") (OtherComp :type "PrimitiveComponent Object Reference") (OtherBodyIndex :type Integer))
  (if (not (`self.Complete`))
    (set `self.Complete` true)
    (`KismetSystemLibrary.PrintString` "플레이어가 범위 밖으로 나갔습니다.")
    (`KismetSystemLibrary.Delay` 5.0)
    (`Widget.RemoveFromParent` (stale `self.Box.OnComponentBeginOverlap` _returnvalue))
    (`KismetSystemLibrary.Delay` 3.0)
    (bind _returnvalue (`|CreateWidget` "/Game/Blueprints/BP_GameComplete.BP_GameComplete_C"))
    (`UserWidget.AddToViewport` _returnvalue 0)
    (`GameplayStatics.SetGamePaused` true)
    (`WidgetBlueprintLibrary.SetInputMode_UIOnlyEx` (`GameplayStatics.GetPlayerController` 0) _returnvalue)
    (set `PlayerController.bShowMouseCursor` true (`GameplayStatics.GetPlayerController` 0))))

(fn `UserConstructionScript`)
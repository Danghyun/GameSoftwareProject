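; BP_PressureSwitch is a pressure plate that operates a door when an actor tagged "Cube" rests on it.
; On overlap it calls SwitchActivated on the first BP_Door found in the level and plays a timeline that moves the switch mesh along Z.
; When any overlap ends, without a tag check, it calls SwitchDeactivated, prints a debug message and reverses the timeline.
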(event `self.ReceiveActorBeginOverlap`
  (params (OtherActor :type "Actor Object Reference"))
  (if (`self.ActorHasTag` OtherActor "Cube")
    (bind _returnvalue (`GameplayStatics.GetActorOfClass` "/Game/Blueprints/BP_Door.BP_Door_C"))
    (`/Game/Blueprints/BP_Door.SwitchActivated` _returnvalue)
    (bind (_direction _switchposition) (`Timeline|SwitchActivate` :!label _label)
      (:`Update`
        (`SceneComponent.K2_SetRelativeLocation` (`self.Switch`) (`KismetMathLibrary.MakeVector` 0.0 0.0 _switchposition) false false)))))

(event `self.ReceiveActorEndOverlap`
  (params (OtherActor :type "Actor Object Reference"))
  (`KismetSystemLibrary.PrintString` "문 닫힘")
  (bind _returnvalue (`GameplayStatics.GetActorOfClass` "/Game/Blueprints/BP_Door.BP_Door_C"))
  (`/Game/Blueprints/BP_Door.SwitchDeactivated` _returnvalue)
  (goto _label :!via `Reverse`))

(fn `UserConstructionScript`)
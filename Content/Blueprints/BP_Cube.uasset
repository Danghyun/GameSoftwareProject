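; BP_Cube is a cube actor that follows in front of the player character while the player is pushing.
; BeginPlay caches the BP_Player instance, and Tick polls its CheckIsPush every frame.
; When true, it moves without sweep to the character's XY plus forward vector times SetLocation, offsetting its own Z by that vector's Z component.
; The cube itself makes no proximity check, and its overlap event is empty.
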(event `self.ReceiveBeginPlay`
  (bind _returnvalue (`GameplayStatics.GetActorOfClass` "/Game/Blueprints/BP_Player.BP_Player_C"))
  (set `self.BP_Player` _returnvalue))

(event `self.ReceiveTick`
  (params (DeltaSeconds :type "Float (single-precision)"))
  (bind (_returnvalue_x _returnvalue_y _returnvalue_z) (`KismetMathLibrary.BreakVector` (`self.K2_GetActorLocation`)))
  (bind _returnvalue (`GameplayStatics.GetPlayerCharacter` 0))
  (bind _returnvalue_2 (`GameplayStatics.GetPlayerCharacter` 0))
  (bind (_returnvalue_x_2 _returnvalue_y_2 _returnvalue_z_2) (`KismetMathLibrary.BreakVector` (`self.GetActorForwardVector` (`GameplayStatics.GetPlayerCharacter` 0))))
  (bind _returnvalue_x_3 (`KismetMathLibrary.BreakVector` (`self.K2_GetActorLocation` _returnvalue_2)))
  (bind _returnvalue_x_4 (`KismetMathLibrary.BreakVector` (`self.GetActorForwardVector` _returnvalue_2)))
  (bind (_returnvalue_x_5 _returnvalue_y_3) (`KismetMathLibrary.BreakVector` (`self.K2_GetActorLocation` _returnvalue)))
  (bind (_returnvalue_x_6 _returnvalue_y_4) (`KismetMathLibrary.BreakVector` (`self.GetActorForwardVector` _returnvalue)))
  (bind _ispush (`/Game/Blueprints/BP_Player.CheckIsPush` (`self.BP_Player`)))
  (if _ispush
    (`self.K2_SetActorLocation` (`KismetMathLibrary.MakeVector` (+ _returnvalue_x_3 (* _returnvalue_x_4 (`self.set location`))) (+ _returnvalue_y_3 (* _returnvalue_y_4 (`self.set location`))) (+ _returnvalue_z (* _returnvalue_z_2 (`self.set location`)))))))

(fn `UserConstructionScript`)